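; BP_NPC_Intro is a scripted intro NPC that moves to a point, holds a dialogue, moves to a second point and destroys itself.
; On BeginPlay it runs Init, retries until the player pawn is a GhostPawn, then waits longer if that pawn uses the intro animation.
; NextAction advances an action counter to select each step; only the first call originates in this graph.
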(event EventBeginPlay
  (Utilities|FlowControl|Sequence
    (:then_0
      (CallFunction|Init))
    (:then_1
      (bind _asghost_pawn (Utilities|Casting|CastToGhostPawn (Game|Player|GetPlayerPawn 0) :!label _label)
        (:then
          (if (Variables|/Game/Blueprints/Player/GhostPawn.GhostPawn_C|GetuseIntroAnim _asghost_pawn)
            (Utilities|FlowControl|Delay 37.0)
            (else
              (Utilities|FlowControl|Delay 1.0)))
          (CallFunction|NextAction))
        (:CastFailed
          (Utilities|FlowControl|Delay 0.1)
          (goto _label))))))

(event EventNextAction
  (bind _actionnum (Variables|Default|GetActionNum))
  (Math|Integer|IncrementInt _actionnum
    (:%20%20
      (switch int _actionnum
        (:0
          (CallFunction|Action-MovetoPoint))
        (:1
          (CallFunction|Action-BeginDialogue))
        (:2
          (CallFunction|Action-MovetoPoint 1))
        (:3
          (Actor|DestroyActor))))))

(fn ConstructionScript)