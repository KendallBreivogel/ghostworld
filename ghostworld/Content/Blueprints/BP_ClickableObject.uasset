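; BP_ClickableObject is a clickable world object, shown as either a static mesh or a Paper2D sprite, that the player can examine or keep.
; Hovering shows its name on the GhostPawn HUD and switches to a grab-hand cursor.
; With CloseInteraction set, clicking turns the character toward it and starts dialogue naming it, or saying too far away beyond InteractionDistance.
; Keepable objects in range also lock the pawn and add keep-item response buttons.
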(event OnClicked(PaperSprite)
  (params (TouchedComponent :type Primitive%20Component%20Object%20Reference) (ButtonPressed :type Key%20Structure :default "None"))
  ;[1 1 1] Click/Mouse Over events
  (if (Variables|Default|GetCloseInteraction)
    (bind _asghost_pawn (Utilities|Casting|CastToGhostPawn (Game|Player|GetPlayerPawn 0)))
    (if (not (Variables|/Game/Blueprints/Player/GhostPawn.GhostPawn_C|GetisOccupied _asghost_pawn))
      (Default|OrienttoLocation (Variables|/Game/Blueprints/Player/GhostPawn.GhostPawn_C|GetCharacter _asghost_pawn) (Transformation|GetActorLocation))
      (if (<= (Transformation|GetDistanceTo (Variables|/Game/Blueprints/Player/GhostPawn.GhostPawn_C|GetCharacter _asghost_pawn) self) (Variables|Default|GetInteractionDistance))
        (if (Variables|Default|GetCanKeep)
          (CallFunction|AddKeepReponses)
          (Default|InitiateDialogue (Variables|/Game/Blueprints/Player/GhostPawn.GhostPawn_C|GetCharacter _asghost_pawn))
          (Default|Dialogue-NameObject (Variables|/Game/Blueprints/Player/GhostPawn.GhostPawn_C|GetCharacter _asghost_pawn) (Variables|Default|GetName))
          (else
            (Default|InitiateDialogue (Variables|/Game/Blueprints/Player/GhostPawn.GhostPawn_C|GetCharacter _asghost_pawn))
            (Default|Dialogue-NameObject (Variables|/Game/Blueprints/Player/GhostPawn.GhostPawn_C|GetCharacter _asghost_pawn) (Variables|Default|GetName))))
        (else
          (Default|InitiateDialogue (Variables|/Game/Blueprints/Player/GhostPawn.GhostPawn_C|GetCharacter _asghost_pawn))
          (Default|Dialogue-TooFarAway (Variables|/Game/Blueprints/Player/GhostPawn.GhostPawn_C|GetCharacter _asghost_pawn)))))))

(event OnBeginCursorOver(PaperSprite)
  (params (TouchedComponent :type Primitive%20Component%20Object%20Reference))
  ;[1 1 1] Click/Mouse Over events
  (bind _asghost_pawn (Utilities|Casting|CastToGhostPawn (Game|Player|GetPlayerPawn 0)))
  (if (not (Variables|/Game/Blueprints/Player/GhostPawn.GhostPawn_C|GetisOccupied _asghost_pawn))
    (Rendering|Components|TextRender|SetText (Variables|/Game/Blueprints/UI/HUD.HUD_C|GetInteractionName (Variables|/Game/Blueprints/Player/GhostPawn.GhostPawn_C|GetHUD _asghost_pawn)) (Utilities|Text|ToText(String) (Variables|Default|GetName)))
    (bind _asghost_controller (Utilities|Casting|CastToGhostController (Game|GetPlayerController 0)))
    (Variables|/Script/Engine.PlayerController|SetCurrentMouseCursor _asghost_controller "GrabHand")))

(event OnEndCursorOver(PaperSprite)
  (params (TouchedComponent :type Primitive%20Component%20Object%20Reference))
  ;[1 1 1] Click/Mouse Over events
  (bind _asghost_pawn (Utilities|Casting|CastToGhostPawn (Game|Player|GetPlayerPawn 0)))
  (if (not (Variables|/Game/Blueprints/Player/GhostPawn.GhostPawn_C|GetisOccupied _asghost_pawn))
    (Rendering|Components|TextRender|SetText (Variables|/Game/Blueprints/UI/HUD.HUD_C|GetInteractionName (Variables|/Game/Blueprints/Player/GhostPawn.GhostPawn_C|GetHUD _asghost_pawn)) (Utilities|Text|ToText(String) ""))
    (bind _asghost_controller (Utilities|Casting|CastToGhostController (Game|GetPlayerController 0)))
    (Variables|/Script/Engine.PlayerController|SetCurrentMouseCursor _asghost_controller "Default")))

(event OnBeginCursorOver(StaticMesh)
  (params (TouchedComponent :type Primitive%20Component%20Object%20Reference))
  ;[1 1 1] Click/Mouse Over events
  (bind _asghost_pawn (Utilities|Casting|CastToGhostPawn (Game|Player|GetPlayerPawn 0)))
  (if (not (Variables|/Game/Blueprints/Player/GhostPawn.GhostPawn_C|GetisOccupied _asghost_pawn))
    (Rendering|Components|TextRender|SetText (Variables|/Game/Blueprints/UI/HUD.HUD_C|GetInteractionName (Variables|/Game/Blueprints/Player/GhostPawn.GhostPawn_C|GetHUD _asghost_pawn)) (Utilities|Text|ToText(String) (Variables|Default|GetName)))
    (bind _asghost_controller (Utilities|Casting|CastToGhostController (Game|GetPlayerController 0)))
    (Variables|/Script/Engine.PlayerController|SetCurrentMouseCursor _asghost_controller "GrabHand")))

(event OnEndCursorOver(StaticMesh)
  (params (TouchedComponent :type Primitive%20Component%20Object%20Reference))
  ;[1 1 1] Click/Mouse Over events
  (bind _asghost_pawn (Utilities|Casting|CastToGhostPawn (Game|Player|GetPlayerPawn 0)))
  (if (not (Variables|/Game/Blueprints/Player/GhostPawn.GhostPawn_C|GetisOccupied _asghost_pawn))
    (Rendering|Components|TextRender|SetText (Variables|/Game/Blueprints/UI/HUD.HUD_C|GetInteractionName (Variables|/Game/Blueprints/Player/GhostPawn.GhostPawn_C|GetHUD _asghost_pawn)) (Utilities|Text|ToText(String) ""))
    (bind _asghost_controller (Utilities|Casting|CastToGhostController (Game|GetPlayerController 0)))
    (Variables|/Script/Engine.PlayerController|SetCurrentMouseCursor _asghost_controller "Default")))

(event OnClicked(StaticMesh)
  (params (TouchedComponent :type Primitive%20Component%20Object%20Reference) (ButtonPressed :type Key%20Structure :default "None"))
  ;[1 1 1] Click/Mouse Over events
  (if (Variables|Default|GetCloseInteraction)
    (bind _asghost_pawn (Utilities|Casting|CastToGhostPawn (Game|Player|GetPlayerPawn 0)))
    (if (not (Variables|/Game/Blueprints/Player/GhostPawn.GhostPawn_C|GetisOccupied _asghost_pawn))
      (Default|OrienttoLocation (Variables|/Game/Blueprints/Player/GhostPawn.GhostPawn_C|GetCharacter _asghost_pawn) (Transformation|GetActorLocation))
      (if (<= (Transformation|GetDistanceTo (Variables|/Game/Blueprints/Player/GhostPawn.GhostPawn_C|GetCharacter _asghost_pawn) self) (Variables|Default|GetInteractionDistance))
        (if (Variables|Default|GetCanKeep)
          (CallFunction|AddKeepReponses)
          (Default|InitiateDialogue (Variables|/Game/Blueprints/Player/GhostPawn.GhostPawn_C|GetCharacter _asghost_pawn))
          (Default|Dialogue-NameObject (Variables|/Game/Blueprints/Player/GhostPawn.GhostPawn_C|GetCharacter _asghost_pawn) (Variables|Default|GetName))
          (else
            (Default|InitiateDialogue (Variables|/Game/Blueprints/Player/GhostPawn.GhostPawn_C|GetCharacter _asghost_pawn))
            (Default|Dialogue-NameObject (Variables|/Game/Blueprints/Player/GhostPawn.GhostPawn_C|GetCharacter _asghost_pawn) (Variables|Default|GetName))))
        (else
          (Default|InitiateDialogue (Variables|/Game/Blueprints/Player/GhostPawn.GhostPawn_C|GetCharacter _asghost_pawn))
          (Default|Dialogue-TooFarAway (Variables|/Game/Blueprints/Player/GhostPawn.GhostPawn_C|GetCharacter _asghost_pawn)))))))

(event Custom|AddKeepReponses
  ;[1 1 1] Add player reponses to HUD
  (if (Variables|Default|GetCanKeep)
    (bind _asghost_pawn (Utilities|Casting|CastToGhostPawn (Game|Player|GetPlayerPawn 0)))
    (Variables|/Game/Blueprints/Player/GhostPawn.GhostPawn_C|SetcanMove _asghost_pawn false)
    (Variables|/Game/Blueprints/Player/GhostPawn.GhostPawn_C|SetisOccupied _asghost_pawn true)
    (Default|AddKeepButtons (Variables|/Game/Blueprints/Player/GhostPawn.GhostPawn_C|GetHUD _asghost_pawn) (Variables|Default|GetName) (Variables|Default|GetInventoryItem) self)
    (Default|SetReponsesVisibility (Variables|/Game/Blueprints/Player/GhostPawn.GhostPawn_C|GetHUD _asghost_pawn) true)))

(event EventBeginPlay
  (bind _papersprite (Variables|Default|GetPaperSprite))
  (bind _staticmesh (Variables|Default|GetStaticMesh))
  ;[1 1 1] Init
  (Physics|SetSimulatePhysics (Variables|Default|GetPaperSprite) false)
  (if (Variables|Default|GetUseMesh)
    (Rendering|SetVisibility _staticmesh true false)
    (Collision|SetCollisionEnabled _staticmesh "QueryAndPhysics")
    (else
      (Rendering|SetVisibility _papersprite true false)
      (Collision|SetCollisionEnabled _papersprite "QueryAndPhysics"))))

(fn ConstructionScript
  (bind _staticmesh (Variables|Default|GetStaticMesh))
  (bind _papersprite (Variables|Default|GetPaperSprite))
  (if (Variables|Default|GetUseMesh)
    (Components|StaticMesh|SetStaticMesh (Variables|Default|GetStaticMesh) (Variables|Default|GetMesh))
    (Rendering|SetVisibility _papersprite false false)
    (Collision|SetCollisionEnabled _papersprite "NoCollision")
    (else
      (Rendering|Components|Sprite|SetSprite (Variables|Default|GetPaperSprite) (Variables|Default|GetSprite))
      (Rendering|SetVisibility _staticmesh false false)
      (Collision|SetCollisionEnabled _staticmesh "NoCollision"))))