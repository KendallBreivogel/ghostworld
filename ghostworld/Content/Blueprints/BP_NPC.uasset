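; Flipbook-sprite NPC that talks to the ghost player in an animated thought bubble and can wander along X around its spawn point.
; Proximity shows a one-time message, while clicking locks player movement and runs indexed NPCDialogue entries with HUD responses, advanced through AdvanceDialogue.
; A timer types text with voice blips, treating # as line breaks and & as click-to-continue pauses; clicking skips typing.
; A material parameter flips sprite facing.
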(event OnFinishedPlaying(DialogueBubble)
  (bind _dialoguebubble (Variables|Default|GetDialogueBubble))
  ;[1 1 1] Dialogue end check
  (if (Variables|proximityDialogue|GetstartingDialogue)
    (Variables|proximityDialogue|SetstartingDialogue false)
    (Components|Timeline|SetLooping _dialoguebubble true)
    (Sprite|SetFlipbook _dialoguebubble "/Game/Animations/Generic/Thought/Continue/Thought_Continue.Thought_Continue")
    (Components|Timeline|SetPlayRate _dialoguebubble -1.5)
    (Audio|Components|Audio|Play _dialoguebubble)
    (CallFunction|SlowPrintText)
    (Development|SetHiddeninGame (Variables|Default|GetTextRender) false false)
    (Variables|Default|SetdialogueBubbleIsOpen true)
    (elif (Variables|proximityDialogue|GetendingDialogue)
      (Variables|proximityDialogue|SetendingDialogue false)
      (Development|SetHiddeninGame (Variables|Default|GetDialogueBubble) true false))))

(event OnClicked(Mesh)
  (params (TouchedComponent :type Primitive%20Component%20Object%20Reference) (ButtonPressed :type Key%20Structure :default "None"))
  ;[1 1 1] Trigger and advance dialogue
  (if (Variables|Default|GetclickDialogue)
    (if (Variables|Default|GetisAwaitingAdvancement)
      (Variables|Default|SetslowPrintTempString "")
      (CallFunction|SlowPrintCharacter)
      (Variables|Default|SetisAwaitingAdvancement false)
      (Variables|Default|SetisSlowPrinting true)
      (elif (Variables|Default|GetisSlowPrinting)
        (CallFunction|EndSlowPrinting)
        (elif (Variables|Default|GetdialogueTriggered)
          (if (and (Variables|Default|GetcanRetriggerDialogue) (not (Variables|Default|GetisInDialogue)))
            (if (not (Variables|/Game/Blueprints/Player/GhostPawn.GhostPawn_C|GetisOccupied (Variables|Default|GetGhost))) :!label _label
              (CallFunction|BeginClickedDialogue)))
          (else
            (goto _label)))))))

(event OnBeginCursorOver(Mesh)
  (params (TouchedComponent :type Primitive%20Component%20Object%20Reference))
  ;[1 1 1] Mouse over events
  (bind _asghost_pawn (Utilities|Casting|CastToGhostPawn (Game|Player|GetPlayerPawn 0)))
  (Rendering|Components|TextRender|SetText (Variables|/Game/Blueprints/UI/HUD.HUD_C|GetInteractionName (Variables|/Game/Blueprints/Player/GhostPawn.GhostPawn_C|GetHUD _asghost_pawn)) (Utilities|Text|ToText(String) (Variables|Default|GetNPCName)))
  (bind _asghost_controller (Utilities|Casting|CastToGhostController (Game|GetPlayerController 0)))
  (Variables|/Script/Engine.PlayerController|SetCurrentMouseCursor _asghost_controller "GrabHand"))

(event OnEndCursorOver(Mesh)
  (params (TouchedComponent :type Primitive%20Component%20Object%20Reference))
  ;[1 1 1] Mouse over events
  (bind _asghost_pawn (Utilities|Casting|CastToGhostPawn (Game|Player|GetPlayerPawn 0)))
  (Rendering|Components|TextRender|SetText (Variables|/Game/Blueprints/UI/HUD.HUD_C|GetInteractionName (Variables|/Game/Blueprints/Player/GhostPawn.GhostPawn_C|GetHUD _asghost_pawn)) (Utilities|Text|ToText(String) ""))
  (bind _asghost_controller (Utilities|Casting|CastToGhostController (Game|GetPlayerController 0)))
  (Variables|/Script/Engine.PlayerController|SetCurrentMouseCursor _asghost_controller "Default"))

(event OnComponentBeginOverlap(Box)
  (params (OverlappedComponent :type Primitive%20Component%20Object%20Reference) (OtherActor :type Actor%20Object%20Reference) (OtherComp :type Primitive%20Component%20Object%20Reference) (OtherBodyIndex :type Integer) (bFromSweep :type Boolean) (SweepResult :type Hit%20Result%20Structure%20%28by%20ref%29))
  ;[1 1 1] Proximity Dialogue
  (Utilities|Casting|CastToGhostCharacter OtherActor)
  (if (and (Variables|proximityDialogue|GetproximityDialogue) (not (Variables|proximityDialogue|GetproximityDialogueTriggered)))
    (CallFunction|BeginDialogue)
    (Variables|Default|SetslowPrintString (Variables|proximityDialogue|GetproximityMessage))
    (Variables|proximityDialogue|SetproximityDialogueTriggered true)))

(event OnClicked(DialogueBubble)
  (params (TouchedComponent :type Primitive%20Component%20Object%20Reference) (ButtonPressed :type Key%20Structure :default "None"))
  ;[1 1 1] Trigger and advance dialogue
  (if (Variables|Default|GetclickDialogue)
    (if (Variables|Default|GetisAwaitingAdvancement)
      (Variables|Default|SetslowPrintTempString "")
      (CallFunction|SlowPrintCharacter)
      (Variables|Default|SetisAwaitingAdvancement false)
      (Variables|Default|SetisSlowPrinting true)
      (elif (Variables|Default|GetisSlowPrinting)
        (CallFunction|EndSlowPrinting)
        (elif (Variables|Default|GetdialogueTriggered)
          (if (and (Variables|Default|GetcanRetriggerDialogue) (not (Variables|Default|GetisInDialogue)))
            (if (not (Variables|/Game/Blueprints/Player/GhostPawn.GhostPawn_C|GetisOccupied (Variables|Default|GetGhost))) :!label _label
              (CallFunction|BeginClickedDialogue)))
          (else
            (goto _label)))))))

(event OnComponentEndOverlap(Box)
  (params (OverlappedComponent :type Primitive%20Component%20Object%20Reference) (OtherActor :type Actor%20Object%20Reference) (OtherComp :type Primitive%20Component%20Object%20Reference) (OtherBodyIndex :type Integer))
  ;[1 1 1] Proximity Dialogue
  (Utilities|Casting|CastToGhostCharacter OtherActor)
  (if (and (Variables|proximityDialogue|GetproximityDialogue) (Variables|proximityDialogue|GetproximityDialogueTriggered))
    (Utilities|FlowControl|Delay 1.0)
    (CallFunction|EndDialogue)))

(event Custom|EndDialogue
  (bind _dialoguebubble (Variables|Default|GetDialogueBubble))
  ;[1 1 1] End Dialogue
  (Sprite|SetFlipbook _dialoguebubble "/Game/Animations/Generic/Thought/Start/Thought_Start.Thought_Start")
  (Components|Timeline|SetPlayRate _dialoguebubble -1.0)
  (Components|Timeline|SetLooping _dialoguebubble true)
  (Components|Timeline|PlayfromStart _dialoguebubble)
  (Variables|proximityDialogue|SetendingDialogue true)
  (Variables|Default|SetdialogueBubbleIsOpen false)
  (Development|SetHiddeninGame (Variables|Default|GetTextRender) true false)
  (Utilities|FlowControl|Delay 1.0)
  (Components|Timeline|SetLooping (Variables|Default|GetDialogueBubble) false))

(event Custom|BeginDialogue
  (bind _dialoguebubble (Variables|Default|GetDialogueBubble))
  ;[1 1 1] BeginDialogue
  (Development|SetHiddeninGame _dialoguebubble false false)
  (Sprite|SetFlipbook _dialoguebubble "/Game/Animations/Generic/Thought/Start/Thought_Start.Thought_Start")
  (Components|Timeline|SetLooping _dialoguebubble false)
  (Audio|Components|Audio|Play _dialoguebubble)
  (Components|Timeline|SetPlayRate _dialoguebubble 4.0)
  (Variables|proximityDialogue|SetstartingDialogue true)
  (Variables|proximityDialogue|SetendingDialogue false))

(event Custom|NextAction)

(event Custom|BeginWandering
  ;[1 1 1] Wander
  (bind _returnvalue (Utilities|Time|SetTimerbyEvent (delegate Custom|WanderRL) (Math|Random|RandomFloatinRange 2.0 8.0)))
  (Variables|Default|SetWanderTimer _returnvalue))

(event Custom|BeginClickedDialogue
  (bind _npcdialogue (Variables|Default|GetNPCDialogue))
  (bind _output (Utilities|Array|Get(acopy) _npcdialogue))
  (bind (_saystring _playerresponses) (Utilities|Struct|BreakNPCDialogue _output))
  ;[1 1 1] Trigger and advance dialogue
  (bind _asghost_pawn (Utilities|Casting|CastToGhostPawn (Game|Player|GetPlayerPawn 0)))
  (Variables|/Game/Blueprints/Player/GhostPawn.GhostPawn_C|SetCurrentNPC _asghost_pawn self)
  (bind _output_get (Variables|Default|SetGhost _asghost_pawn))
  (Variables|/Game/Blueprints/Player/GhostPawn.GhostPawn_C|SetisOccupied _output_get true)
  (Variables|Default|SetisInDialogue true)
  (Variables|Default|SetdialogueTriggered true)
  (Variables|/Game/Blueprints/Player/GhostPawn.GhostPawn_C|SetcanMove (Variables|Default|GetGhost) false)
  (Default|OrienttoLocation (Variables|/Game/Blueprints/Player/GhostPawn.GhostPawn_C|GetCharacter (Variables|Default|GetGhost)) (Transformation|GetActorLocation))
  (CallFunction|OrienttoLocation (Transformation|GetActorLocation (Variables|/Game/Blueprints/Player/GhostPawn.GhostPawn_C|GetCharacter (Variables|Default|GetGhost))))
  (Default|WipeReponses (Variables|/Game/Blueprints/Player/GhostPawn.GhostPawn_C|GetHUD (Variables|Default|GetGhost)))
  (Default|AddReponses (Variables|/Game/Blueprints/Player/GhostPawn.GhostPawn_C|GetHUD (Variables|Default|GetGhost)) _playerresponses)
  (Variables|Default|SetslowPrintString _saystring)
  (Utilities|Time|ClearandInvalidateTimerbyHandle (Variables|Default|GetWanderTimer))
  (Default|SetReponsesVisibility (Variables|/Game/Blueprints/Player/GhostPawn.GhostPawn_C|GetHUD (Variables|Default|GetGhost)) false)
  (if (Variables|Default|GetdialogueBubbleIsOpen)
    (CallFunction|SlowPrintText)
    (else
      (CallFunction|BeginDialogue))))

(event Custom|orientToLocation
  (params (Location :type Vector))
  (bind _flipbookmat (Variables|Default|GetFlipbookMat))
  ;[1 1 1] Orient to location
  (if (> (.X (Math|Vector|BreakVector Location)) (.x (Transformation|GetActorLocation)))
    (Rendering|Material|SetScalarParameterValue _flipbookmat "X" 1.0 :!class /Script/Engine.MaterialInstanceDynamic)
    (else
      (Rendering|Material|SetScalarParameterValue _flipbookmat "X" -1.0 :!class /Script/Engine.MaterialInstanceDynamic))))

(event Custom|AdvanceDialogue
  (params (GoTo :type Integer))
  (bind _npcdialogue (Variables|Default|GetNPCDialogue))
  (bind _ghost (Variables|Default|GetGhost))
  (bind _ghost_2 (Variables|Default|GetGhost))
  (bind _output (Utilities|Array|Get(acopy) _npcdialogue GoTo))
  (bind _hud (Variables|/Game/Blueprints/Player/GhostPawn.GhostPawn_C|GetHUD _ghost_2))
  (bind (_saystring _playerresponses) (Utilities|Struct|BreakNPCDialogue _output))
  ;[1 1 1] Trigger and advance dialogue
  (if (== GoTo -1)
    (CallFunction|EndDialogue)
    (Variables|Default|SetisInDialogue false)
    (Variables|/Game/Blueprints/Player/GhostPawn.GhostPawn_C|SetcanMove _ghost true)
    (Variables|/Game/Blueprints/Player/GhostPawn.GhostPawn_C|SetisOccupied _ghost false)
    (Default|WipeReponses (Variables|/Game/Blueprints/Player/GhostPawn.GhostPawn_C|GetHUD _ghost))
    (CallFunction|NextAction)
    (if (Variables|Default|GetWander)
      (CallFunction|BeginWandering))
    (else
      (Default|WipeReponses _hud)
      (Default|AddReponses _hud _playerresponses)
      (Variables|Default|SetslowPrintString _saystring)
      (CallFunction|SlowPrintText)
      (Default|SetReponsesVisibility (Variables|/Game/Blueprints/Player/GhostPawn.GhostPawn_C|GetHUD (Variables|Default|GetGhost)) false))))

(event Custom|SlowPrintText
  ;[1 1 1] Slow printing, skipping, and sentence advancement
  (Rendering|Components|TextRender|SetText (Variables|Default|GetTextRender) (Utilities|Text|ToText(String) ""))
  (Variables|Default|SetslowPrintTempString "")
  (Variables|Default|SetslowPrintInt 0)
  (Variables|Default|Set&num 0)
  (Variables|Default|SetisSlowPrinting true)
  (bind _returnvalue (Utilities|Time|SetTimerbyEvent (delegate Custom|SlowPrintCharacter) 0.1))
  (Variables|Default|SetslowPrintTimer _returnvalue))

(event Custom|SlowPrintCharacter
  (bind _slowprintstring (Variables|Default|GetslowPrintString))
  (bind _slowprintint (Variables|Default|GetslowPrintInt))
  (bind _returnvalue (Utilities|String|GetSubstring _slowprintstring _slowprintint))
  ;[1 1 1] Slow printing, skipping, and sentence advancement
  (Audio|PlaySound2D "/Game/Audio/Bass/Bass.Bass" (/ (Math|Conversions|ToFloat(Integer) (Math|Integer|%(Integer) (Variables|Default|GetslowPrintInt) 2)) 2.5) (Variables|Default|GetVoicePitch) 0.0 0 0)
  (if (<= (Variables|Default|GetslowPrintInt) (Utilities|String|Len _slowprintstring))
    (if (Utilities|Enum|Equal(Enum) _returnvalue "#")
      (Variables|Default|SetslowPrintTempString (Utilities|String|Append (Variables|Default|GetslowPrintTempString) "<br>"))
      (Rendering|Components|TextRender|SetText (Variables|Default|GetTextRender) (Utilities|Text|ToText(String) (Variables|Default|GetslowPrintTempString)) :!label _label)
      (Math|Integer|IncrementInt (Variables|Default|GetslowPrintInt)
        (:%20%20
          (bind _returnvalue_2 (Utilities|Time|SetTimerbyEvent (delegate Custom|SlowPrintCharacter) 0.05))
          (Variables|Default|SetslowPrintTimer _returnvalue_2)))
      (elif (Utilities|Enum|Equal(Enum) _returnvalue "&")
        (Math|Integer|IncrementInt (Variables|Default|GetslowPrintInt)
          (:%20%20
            (Math|Integer|IncrementInt (Variables|Default|Get&num)
              (:%20%20
                (Variables|Default|SetisAwaitingAdvancement true)))))
        (else
          (Variables|Default|SetslowPrintTempString (Utilities|String|Append (Variables|Default|GetslowPrintTempString) _returnvalue))
          (goto _label))))
    (else
      (Variables|Default|SetisSlowPrinting false)
      (Default|SetReponsesVisibility (Variables|/Game/Blueprints/Player/GhostPawn.GhostPawn_C|GetHUD (Variables|Default|GetGhost)) true))))

(event Custom|Init
  ;[1 1 1] Init
  (Variables|Default|SetStartingLocation (Transformation|GetActorLocation))
  (Utilities|FlowControl|Sequence
    (:then_0
      (bind _asghost_pawn (Utilities|Casting|CastToGhostPawn (Game|Player|GetPlayerPawn 0)))
      (Variables|Default|SetGhost _asghost_pawn))
    (:then_1
      (if (Variables|Default|GetWander)
        (CallFunction|BeginWandering)))))

(event Custom|ParseSlowString
  (params (BeginAt :type Integer))
  (bind _slowprintstring (Variables|Default|GetslowPrintString))
  ;[1 1 1] Slow printing, skipping, and sentence advancement
  (Variables|Default|SetslowPrintTempString "")
  (bind _index (Utilities|FlowControl|ForLoopwithBreak BeginAt (- (Utilities|String|Len _slowprintstring) 1) :!label _label)
    (:LoopBody
      (if (Utilities|Enum|Equal(Enum) (Utilities|String|GetSubstring _slowprintstring _index) "#")
        (Variables|Default|SetslowPrintTempString (Utilities|String|Append (Variables|Default|GetslowPrintTempString) "<br>"))
        (elif (Utilities|Enum|Equal(Enum) (Utilities|String|GetSubstring _slowprintstring _index) "&")
          (Variables|Default|SetisAwaitingAdvancement true)
          (Math|Integer|IncrementInt (Variables|Default|Get&num)
            (:%20%20
              (Variables|Default|SetslowPrintInt (+ _index 1))
              (goto _label Break)))
          (else
            (Variables|Default|SetslowPrintTempString (Utilities|String|Append (Variables|Default|GetslowPrintTempString) (Utilities|String|GetSubstring _slowprintstring _index)))))))
    (:Completed
      (Rendering|Components|TextRender|SetText (Variables|Default|GetTextRender) (Utilities|Text|ToText(String) (Variables|Default|GetslowPrintTempString))))))

(event Custom|WanderRL
  (bind _wanderdist (Variables|Default|GetWanderDist))
  (bind _startinglocation (Variables|Default|GetStartingLocation))
  ;[1 1 1] Wander
  (bind _output_get (Variables|Default|SetWanderLocation (Math|Vector|MakeVector (+ (.x _startinglocation) (Math|Random|RandomFloatinRange (* _wanderdist -1.0) _wanderdist)) (.y _startinglocation) (.z _startinglocation))))
  (CallFunction|OrienttoLocation _output_get)
  (AI|AIMoveTo self (Variables|Default|GetWanderLocation) 0 1.0 true
    (:OnSuccess
      _)
    (:OnFail
      _))
  (bind _returnvalue (Utilities|Time|SetTimerbyEvent (delegate Custom|WanderRL) (Math|Random|RandomFloatinRange 2.0 8.0)))
  (Variables|Default|SetWanderTimer _returnvalue))

(event Custom|EndSlowPrinting
  ;[1 1 1] Slow printing, skipping, and sentence advancement
  (bind _beginat (CallFunction|GetParseSlowStringStartingPoint))
  (CallFunction|ParseSlowString _beginat)
  (Variables|Default|SetisSlowPrinting false)
  (Utilities|FlowControl|Sequence
    (:then_0
      (Utilities|Time|ClearandInvalidateTimerbyHandle (Variables|Default|GetslowPrintTimer)))
    (:then_1
      (if (not (Variables|Default|GetisAwaitingAdvancement))
        (Default|SetReponsesVisibility (Variables|/Game/Blueprints/Player/GhostPawn.GhostPawn_C|GetHUD (Variables|Default|GetGhost)) true)))))

(event EventBeginPlay
  (CallFunction|Init))

(fn ConstructionScript
  (Rendering|Components|TextRender|SetText (Variables|Default|GetTextRender) (Utilities|Text|ToText(String) (Variables|proximityDialogue|GetproximityMessage)))
  (Transformation|SetRelativeScale3D (Variables|Default|GetBox) (Variables|proximityDialogue|GetproximityVolSize))
  (bind _returnvalue (Rendering|Material|CreateDynamicMaterialInstance "/Game/Materials/M_Flipbook.M_Flipbook" "None" :!class /Script/Engine.KismetMaterialLibrary))
  (bind _output_get (Variables|Default|SetFlipbookMat _returnvalue))
  (Rendering|Material|SetMaterial (Variables|Character|GetMesh) 0 _output_get))

(fn GetParseSlowStringStartingPoint
  (bind __num (Variables|Default|Get&num))
  (Variables|Default|Set&numLoc 0)
  (if (> __num 0)
    (Variables|Default|Set&numTempString (Variables|Default|GetslowPrintString))
    (for _index (range 0 __num)
      (Variables|Default|Set&numLoc (+ (Variables|Default|Get&numLoc) (+ (Utilities|String|FindSubstring (Variables|Default|Get&numTempString) "&") 1)))
      (Variables|Default|Set&numTempString (Utilities|String|GetSubstring (Variables|Default|Get&numTempString) (+ (Utilities|String|FindSubstring (Variables|Default|Get&numTempString) "&") 1) (- (Utilities|String|Len (Variables|Default|Get&numTempString)) (+ (Utilities|String|FindSubstring (Variables|Default|Get&numTempString) "&") 1)))))
    (return (Variables|Default|Get&numLoc))
    (else
      (return 0))))