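; Player ghost character that moves to requested floor points and voices randomized remarks in an animated thought bubble.
; Movement uses AIMoveTo, mirrors the mesh on X to face the target, and shows a spawned banner at the destination until the move ends.
; The flipbook bubble chains open, loop and close animations through OnFinishedPlaying and state flags, with a restartable timer to auto-close it.
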(event OnFinishedPlaying(DialogueBubble)
  (bind _dialoguebubble (Variables|Default|GetDialogueBubble))
  ;[1 1 1] Dialogue end check
  (if (Variables|Default|GetstartingDialogue)
    (Variables|Default|SetstartingDialogue false)
    (Components|Timeline|SetLooping _dialoguebubble true)
    (Sprite|SetFlipbook _dialoguebubble "/Game/Animations/Generic/Thought/Continue/Thought_Continue.Thought_Continue")
    (Components|Timeline|SetPlayRate _dialoguebubble -1.5)
    (Audio|Components|Audio|Play _dialoguebubble)
    (Development|SetHiddeninGame (Variables|Default|GetTextRender) false false)
    (elif (Variables|Default|GetendingDialogue)
      (Variables|Default|SetendingDialogue false)
      (Development|SetHiddeninGame (Variables|Default|GetDialogueBubble) true false)
      (Variables|Default|SetDialogueBubbleIsOpen false))))

(event Custom|EndDialogue
  (bind _dialoguebubble (Variables|Default|GetDialogueBubble))
  ;[1 1 1] End Dialogue
  (Sprite|SetFlipbook _dialoguebubble "/Game/Animations/Generic/Thought/Start/Thought_Start.Thought_Start")
  (Components|Timeline|SetPlayRate _dialoguebubble -4.0)
  (Components|Timeline|SetLooping _dialoguebubble true)
  (Components|Timeline|PlayfromStart _dialoguebubble)
  (Variables|Default|SetendingDialogue true)
  (Development|SetHiddeninGame (Variables|Default|GetTextRender) true false)
  (Utilities|FlowControl|Delay 0.25)
  (Components|Timeline|SetLooping (Variables|Default|GetDialogueBubble) false))

(event Custom|BeginDialogue
  (bind _dialoguebubble (Variables|Default|GetDialogueBubble))
  ;[1 1 1] BeginDialogue
  (Development|SetHiddeninGame _dialoguebubble false false)
  (Sprite|SetFlipbook _dialoguebubble "/Game/Animations/Generic/Thought/Start/Thought_Start.Thought_Start")
  (Components|Timeline|SetLooping _dialoguebubble false)
  (Audio|Components|Audio|Play _dialoguebubble)
  (Components|Timeline|SetPlayRate _dialoguebubble 8.0)
  (Variables|Default|SetstartingDialogue true)
  (Variables|Default|SetendingDialogue false)
  (Variables|Default|SetDialogueBubbleIsOpen true))

(event Custom|orientToLocation
  (params (Location :type Vector))
  (bind _mesh (Variables|Character|GetMesh))
  ;[1 1 1] Orient to location
  (if (> (.X (Math|Vector|BreakVector Location)) (.x (Transformation|GetActorLocation)))
    (Transformation|SetRelativeScale3D _mesh "1.000000,1.000000,1.000000")
    (else
      (Transformation|SetRelativeScale3D _mesh "-1.000000,1.000000,1.000000"))))

(event Custom|moveToFloorPoint
  (params (Location :type Vector))
  (bind (_x _y _z) (Math|Vector|BreakVector Location))
  (bind _banner (Variables|Default|GetBanner))
  ;[1 1 1] Move
  (Utilities|FlowControl|Sequence
    (:then_0
      (if (not (Variables|Default|GetEndingDialogue))
        (CallFunction|CloseDialogueBubble)))
    (:then_1
      (AI|AIMoveTo self Location 0 5.0 false
        (:then
          (CallFunction|OrienttoLocation Location)
          (Transformation|SetActorLocation _banner (Math|Vector|MakeVector _x _y (+ _z 25.0)) false false)
          (Rendering|SetActorHiddenInGame _banner false))
        (:OnSuccess
          (Rendering|SetActorHiddenInGame _banner true :!label _label))
        (:OnFail
          (Development|PrintString "Oh no!")
          (goto _label))))))

(event Custom|InitiateDialogue
  ;[1 1 1] Initiate and end dialogue animations
  (if (Variables|Default|GetDialogueBubbleIsOpen)
    (Utilities|Time|ClearandInvalidateTimerbyHandle (Variables|Default|GetCloseDialogueBubbleTimer))
    (else
      (CallFunction|BeginDialogue)))
  (bind _returnvalue (Utilities|Time|SetTimerbyEvent (delegate Custom|CloseDialogueBubble) 2.5))
  (Variables|Default|SetCloseDialogueBubbleTimer _returnvalue))

(event Custom|CloseDialogueBubble
  ;[1 1 1] Initiate and end dialogue animations
  (CallFunction|EndDialogue))

(event Custom|Dialogue-%20NameObject
  (params (Name :type String))
  (bind _textrender (Variables|Default|GetTextRender))
  ;[1 1 1] Dialogue
  (switch int (Math|Random|RandomIntegerinRange 0 3)
    (:0
      (Rendering|Components|TextRender|SetText _textrender (Utilities|Text|ToText(String) (Utilities|String|Append "Just an ordinary<br>" Name "."))))
    (:1
      (Rendering|Components|TextRender|SetText _textrender (Utilities|Text|ToText(String) (Utilities|String|Append "Its a <br>" Name "."))))
    (:2
      (Rendering|Components|TextRender|SetText _textrender (Utilities|Text|ToText(String) (Utilities|String|Append "Hey, a <br>" Name "."))))
    (:3
      (Rendering|Components|TextRender|SetText _textrender (Utilities|Text|ToText(String) (Utilities|String|Append "...a<br>" Name "."))))))

(event Custom|Dialogue-%20TooFarAway
  (bind _textrender (Variables|Default|GetTextRender))
  ;[1 1 1] Dialogue
  (switch int (Math|Random|RandomIntegerinRange 0 2)
    (:0
      (Rendering|Components|TextRender|SetText _textrender (Utilities|Text|ToText(String) "I need to <br>get closer.")))
    (:1
      (Rendering|Components|TextRender|SetText _textrender (Utilities|Text|ToText(String) "Too far away...")))
    (:2
      (Rendering|Components|TextRender|SetText _textrender (Utilities|Text|ToText(String) "I'm not close <br>enough to that.")))))

(event EventBeginPlay
  ;[1 1 1] Init
  (bind _returnvalue (Game|SpawnActorfromClass "/Game/Blueprints/Player/BP_MoveBanner.BP_MoveBanner_C" (Math|Transform|MakeTransform "0, 0, 0" "0, 0, 0" "0.100000,0.100000,0.100000") "Undefined" 0 0))
  (Variables|Default|SetBanner _returnvalue))

(fn ConstructionScript)