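; Player pawn that controls a separately spawned AI GhostCharacter through click-to-move and owns the inventory and HUD.
; An optional intro switches the view to a tagged cinematic actor, then swaps in the ghost after timed delays.
; Left-click traces under the cursor and sends floor hits to the ghost.
; A looping timer slides the inventory bar when the cursor enters or leaves the top screen edge; added items refresh the capped inventory.
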(event Custom|IntroAnim
  (bind _character (Variables|Default|GetCharacter))
  ;[1 1 1] Intro Animation
  (Utilities|FlowControl|Delay 0.1)
  (Variables|Default|SetcanMove false)
  (Rendering|SetActorHiddenInGame (Variables|Default|GetCharacter) true)
  (bind _outactors (Actor|GetAllActorswithTag "IntroAnim"))
  (bind _output_get (Variables|Default|SetintroAnimCharacter (Utilities|Array|Get(acopy) _outactors)))
  (bind _asbp_intro_anim_character (Utilities|Casting|CastToBP_IntroAnimCharacter _output_get))
  (Game|Player|SetViewTargetwithBlend (Game|GetPlayerController 0) (Variables|/Game/Blueprints/BP_IntroAnimCharacter.BP_IntroAnimCharacter_C|GetCamera _asbp_intro_anim_character) 0.01 "VTBlend_Linear" 0.0 false)
  (Utilities|FlowControl|Delay 25.700001)
  (Utilities|FlowControl|Sequence
    (:then_0
      (Utilities|FlowControl|Delay 3.0)
      (Audio|Components|Audio|Play (Variables|/Game/Blueprints/BP_IntroAnimCharacter.BP_IntroAnimCharacter_C|GetSkeletalMesh _asbp_intro_anim_character) false)
      (Utilities|FlowControl|Delay 8.292)
      (Transformation|SetActorLocation _character (Math|Vector|MakeVector (.x (Transformation|GetActorLocation _output_get)) (.y (Transformation|GetActorLocation _output_get)) (+ (.z (Transformation|GetActorLocation _output_get)) 8e+01)) false false)
      (Rendering|SetActorHiddenInGame _output_get true)
      (Rendering|SetActorHiddenInGame _character false)
      (Variables|Default|SetcanMove true)
      (CallFunction|BeginCheckingCursorPos))
    (:then_1
      (Game|Player|SetViewTargetwithBlend (Game|GetPlayerController 0) self 0.0 "VTBlend_Linear" 0.0 false))))

(event Custom|ItemSelected
  (params (itemNum :type Integer)))

(event Custom|CheckCursorPos
  (bind _hud (Variables|Default|GetHUD))
  ;[1 1 1] Check cursor pos
  (bind _returnvalue (Class|WidgetLayoutLibrary|GetMousePositiononViewport))
  (Utilities|FlowControl|Sequence
    (:then_0
      (if (<= (/ (* (.Y (Math|Vector2D|BreakVector2D _returnvalue)) (Class|WidgetLayoutLibrary|GetViewportScale)) (Math|Conversions|ToFloat(Integer) (.SizeY (HUD|GetViewportSize (Game|GetPlayerController 0))))) 0.2)
        (Utilities|FlowControl|DoOnce false :!label _label
          (:Completed
            (Variables|/Game/Blueprints/UI/HUD.HUD_C|SetLerpInventory _hud true)
            (Variables|/Game/Blueprints/UI/HUD.HUD_C|SetTargetInventoryPos _hud 0.0)
            (goto _label_2 Reset)))
        (else
          (Utilities|FlowControl|DoOnce false :!label _label_2
            (:Completed
              (Variables|/Game/Blueprints/UI/HUD.HUD_C|SetLerpInventory _hud true)
              (Variables|/Game/Blueprints/UI/HUD.HUD_C|SetTargetInventoryPos _hud -175.0)
              (goto _label Reset))))))))

(event Custom|beginCheckingCursorPos
  ;[1 1 1] Check cursor pos
  (Utilities|Time|SetTimerbyEvent (delegate Custom|CheckCursorPos) 0.1 true))

(event Custom|AddItemToInventory
  (params (Item :type Inventory%20Item%20Structure))
  ;[1 1 1] Inventory
  (if (< (Utilities|Array|Length (Variables|Default|GetInventory)) 10)
    (Utilities|Array|Add (Variables|Default|GetInventory) Item)
    (Default|UpdateInventory (Variables|Default|GetHUD))))

(event EventBeginPlay
  ;[1 1 1] Init
  (Utilities|FlowControl|Sequence
    (:then_0
      (bind _returnvalue (AI|SpawnAIFromClass "/Game/Blueprints/Player/GhostCharacter.GhostCharacter_C" 0 (.location (Transformation|GetActorTransform)) "0, 0, 0" false))
      (bind _asghost_character (Utilities|Casting|CastToGhostCharacter _returnvalue))
      (Variables|/Game/Blueprints/Player/GhostCharacter.GhostCharacter_C|SetOwningPawn _asghost_character self)
      (Variables|Default|SetCharacter _asghost_character))
    (:then_1
      (bind _returnvalue_2 (UserInterface|CreateWidget "/Game/Blueprints/UI/HUD.HUD_C" 0 self))
      (bind _output_get (Variables|Default|SetHUD _returnvalue_2))
      (UserInterface|Viewport|AddtoPlayerScreen _output_get))
    (:then_2
      (if (Variables|Default|GetuseIntroAnim)
        (CallFunction|IntroAnim)
        (else
          (CallFunction|BeginCheckingCursorPos))))))

(event Collision|EventActorBeginOverlap
  (params (OtherActor :type Actor%20Object%20Reference))
  ;[1 1 1] Init
)

(event EventTick
  (params (DeltaSeconds :type Float%20%28single-precision%29))
  ;[1 1 1] Init
)

(event Input|ActionEvents|InputActionLeftClick
  (params (Key :type Key%20Structure :default "None"))
  ;[1 1 1] Click to move
  (:Pressed
    (if (Variables|Default|GetcanMove)
      (bind _asplayer_controller (Utilities|Casting|CastToPlayerController (Pawn|GetController)))
      (if (.ReturnValue (Game|Player|GetHitResultUnderCursorbyChannel _asplayer_controller "TraceTypeQuery1" true))
        (if (Utilities|Enum|Equal(Enum) (Collision|GetCollisionObjectType (.HitComponent (Collision|BreakHitResult (.HitResult (Game|Player|GetHitResultUnderCursorbyChannel _asplayer_controller "TraceTypeQuery1" true))))) "ECC_GameTraceChannel2")
          (Default|MovetoFloorPoint (Variables|Default|GetCharacter) (.Location (Collision|BreakHitResult (.HitResult (Game|Player|GetHitResultUnderCursorbyChannel _asplayer_controller "TraceTypeQuery1" true))))))))))

(fn ConstructionScript)