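; BP_Poster is a placeable poster actor with a configurable image and height, built from a back plane and a poster plane.
; The construction script creates a dynamic instance of M_Poster, feeds the Poster texture into it and applies it to the poster plane.
; It scales both planes' Y axis from Height, keeping the poster plane slightly smaller than the back plane.
; The event graph has no active logic.
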(event EventBeginPlay)

(event Collision|EventActorBeginOverlap
  (params (OtherActor :type Actor%20Object%20Reference)))

(event EventTick
  (params (DeltaSeconds :type Float%20%28single-precision%29)))

(fn ConstructionScript
  (bind _height (Variables|Default|GetHeight))
  (bind _returnvalue (Rendering|Material|CreateDynamicMaterialInstance "/Game/Materials/M_Poster.M_Poster" "None" :!class /Script/Engine.KismetMaterialLibrary))
  (Rendering|Material|SetTextureParameterValue _returnvalue "Poster" (Variables|Default|GetPoster))
  (Rendering|Material|SetMaterial (Variables|Default|GetPosterPlane) 0 _returnvalue)
  (Transformation|SetRelativeScale3D (Variables|Default|GetBackPlane) (Math|Vector|MakeVector 1.0 _height 1.0))
  (Transformation|SetRelativeScale3D (Variables|Default|GetPosterPlane) (Math|Vector|MakeVector 0.9 (- _height 0.1) 0.9)))