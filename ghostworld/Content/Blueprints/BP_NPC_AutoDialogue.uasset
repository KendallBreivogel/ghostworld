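; BP_NPC_AutoDialogue is an NPC Blueprint that runs actions for walking between points and starting dialogue.
; It calls Init on BeginPlay.
; The move action turns the NPC toward an indexed MoveToPoints actor, sends it there with AIMoveTo, and calls NextAction on success to advance the sequence.
; The dialogue action calls BeginClickedDialogue, reusing the clicked-dialogue entry point.
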(event Custom|Action-Begin%20Dialogue
  (CallFunction|BeginClickedDialogue))

(event Custom|Action-%20Move%20to%20Point
  (params (PointNum :type Integer))
  (bind _movetopoints (Variables|Default|GetMoveToPoints))
  (bind _output (Utilities|Array|Get(acopy) _movetopoints PointNum))
  (bind _returnvalue (Transformation|GetActorLocation _output))
  (CallFunction|OrienttoLocation _returnvalue)
  (AI|AIMoveTo self _returnvalue 0 2.0 true
    (:OnSuccess
      (CallFunction|NextAction))))

(event EventBeginPlay
  (Utilities|FlowControl|Sequence
    (:then_0
      (CallFunction|Init))))

(fn ConstructionScript)