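; BP_IntroAnimCharacter is an intro animation actor that spawns and animates a downward-facing camera, without setting it as the view target itself.
; On BeginPlay it attaches a new CameraActor to its Scene component and plays the slowed Follow timeline.
; Each update shifts Scene's relative height and roll from the timeline value, then copies its world transform to the camera.
; Spline-based position and rotation nodes remain unused.
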(event EventBeginPlay
  (bind _scene (Variables|Default|GetScene))
  (bind _scene_2 (Variables|Default|GetScene))
  (Components|Timeline|SetPlayRate (Variables|Default|GetFollow) 0.2)
  (bind _returnvalue (Game|SpawnActorfromClass "/Script/Engine.CameraActor" (Transformation|GetWorldTransform _scene_2) "Undefined" 0 0))
  (Transformation|AttachComponentToComponent _returnvalue _scene_2 "None" "KeepWorld" "KeepWorld" "KeepWorld" true)
  (Variables|Default|SetCamera _returnvalue)
  (bind _length (Timeline|Follow PlayFromStart)
    (:Update
      (Transformation|SetRelativeLocation _scene (Math|Vector|MakeVector 0.0 -1.5e+02 (+ (* _length 1e+02) 255.0)) false false)
      (Transformation|SetRelativeRotation _scene (Math|Rotator|MakeRotator (+ (* _length 45.0) 1.8e+02) -9e+01 0.0) false false)
      (Transformation|SetActorTransform (Variables|Default|GetCamera) (Transformation|GetWorldTransform _scene)))))

(fn ConstructionScript)