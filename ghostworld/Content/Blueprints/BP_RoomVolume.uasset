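; Room trigger volume that moves the player's ghost pawn to the room's camera point and reveals the room when the ghost character enters.
; Entry lerps the pawn by timeline, swaps collision on hide/display actor lists, restores the previous room's walls and streams configured levels in and out.
; Wall fades use two dynamic materials assigned in the construction script, with opposite opacities driven by one reversible timeline.
; A starting room applies its hidden state shortly after BeginPlay.
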(event OnComponentBeginOverlap(Box)
  (params (OverlappedComponent :type Primitive%20Component%20Object%20Reference) (OtherActor :type Actor%20Object%20Reference) (OtherComp :type Primitive%20Component%20Object%20Reference) (OtherBodyIndex :type Integer) (bFromSweep :type Boolean) (SweepResult :type Hit%20Result%20Structure%20%28by%20ref%29))
  (bind _ghost (Variables|Default|GetGhost))
  (bind _character (Variables|/Game/Blueprints/Player/GhostPawn.GhostPawn_C|GetCharacter _ghost))
  (bind _owningpawn (Variables|/Game/Blueprints/Player/GhostCharacter.GhostCharacter_C|GetOwningPawn _character))
  ;[1 1 1] Overlap triggers
  (Utilities|Casting|CastToGhostCharacter OtherActor)
  (if (Utilities|IsValid _character)
    (Utilities|FlowControl|Sequence
      (:then_0
        (Variables|Default|SetStartingLocation (Transformation|GetActorLocation _owningpawn))
        (bind _lerp (Timeline|LerpCamera PlayFromStart)
          (:Update
            (Transformation|SetActorLocation _owningpawn (Math|Vector|Lerp(Vector) (Variables|Default|GetStartingLocation) (Transformation|GetActorLocation (Variables|Default|GetCameraLocation)) _lerp) false false))
          (:Finished
            (Variables|/Game/Blueprints/Player/GhostPawn.GhostPawn_C|SetCurrentRoom _ghost self))))
      (:then_1
        (CallFunction|HideActors :!label _label))
      (:then_2
        (if (Utilities|IsValid (Variables|/Game/Blueprints/Player/GhostPawn.GhostPawn_C|GetCurrentRoom _ghost))
          (CallFunction|UnhideActors (Variables|/Game/Blueprints/Player/GhostPawn.GhostPawn_C|GetCurrentRoom _ghost))))
      (:then_3
        (CallFunction|Load)
        (CallFunction|Unload)))
    (else
      (goto _label))))

(event OnComponentEndOverlap(Box)
  (params (OverlappedComponent :type Primitive%20Component%20Object%20Reference) (OtherActor :type Actor%20Object%20Reference) (OtherComp :type Primitive%20Component%20Object%20Reference) (OtherBodyIndex :type Integer))
  ;[1 1 1] Overlap triggers
  (Utilities|Casting|CastToGhostCharacter OtherActor))

(event Custom|HideActors
  ;[1 1 1] Hide and show walls
  (Utilities|FlowControl|Sequence
    (:then_0
      (for _array_element (Variables|Default|GetToDisplay)
        (Collision|SetActorEnableCollision _array_element true)))
    (:then_1
      (for _array_element_2 (Variables|Default|GetToHide)
        (Collision|SetActorEnableCollision _array_element_2 false))
      (CallFunction|FadeWallsOut))))

(event Custom|FadeWallsIn
  ;[1 1 1] Hide and show walls
  (bind _opacity (Timeline|FadeOut ReverseFromEnd)
    (:Update
      (Rendering|Material|SetScalarParameterValue (Variables|Default|GetMat_FadeOut) "Opacity" _opacity :!class /Script/Engine.MaterialInstanceDynamic)
      (Rendering|Material|SetScalarParameterValue (Variables|Default|GetMat_FadeIn) "Opacity" (- 1.0 _opacity) :!class /Script/Engine.MaterialInstanceDynamic))))

(event Custom|FadeWallsOut
  ;[1 1 1] Hide and show walls
  (bind _opacity (Timeline|FadeOut PlayFromStart)
    (:Update
      (Rendering|Material|SetScalarParameterValue (Variables|Default|GetMat_FadeOut) "Opacity" _opacity :!class /Script/Engine.MaterialInstanceDynamic)
      (Rendering|Material|SetScalarParameterValue (Variables|Default|GetMat_FadeIn) "Opacity" (- 1.0 _opacity) :!class /Script/Engine.MaterialInstanceDynamic))))

(event Custom|Unload
  (for _array_element (Variables|Default|GetunloadLevels)
    (Game|UnloadStreamLevel(byName) _array_element false)))

(event Custom|UnhideActors
  ;[1 1 1] Hide and show walls
  (Utilities|FlowControl|Sequence
    (:then_0
      (for _array_element (Variables|Default|GetToDisplay)
        (Collision|SetActorEnableCollision _array_element false)))
    (:then_1
      (for _array_element_2 (Variables|Default|GetToHide)
        (Collision|SetActorEnableCollision _array_element_2 true))
      (CallFunction|FadeWallsin))))

(event Custom|Load
  (for _array_element (Variables|Default|GetloadLevels)
    (Game|LoadStreamLevel(byName) _array_element true true)))

(event EventBeginPlay
  ;[1 1 1] Init
  (Utilities|FlowControl|Sequence
    (:then_0
      (if (Variables|Default|GetStartingRoom)
        (Utilities|FlowControl|Delay 0.2)
        (Variables|/Game/Blueprints/Player/GhostPawn.GhostPawn_C|SetCurrentRoom (Variables|Default|GetGhost) self)
        (CallFunction|HideActors)))
    (:then_1
      (bind _asghost_pawn (Utilities|Casting|CastToGhostPawn (Game|Player|GetPlayerPawn 0)))
      (Variables|Default|SetGhost _asghost_pawn))))

(fn ConstructionScript
  (Utilities|FlowControl|Sequence
    (:then_0
      (bind _returnvalue (Rendering|Material|CreateDynamicMaterialInstance "/Game/Materials/M_FadeOut.M_FadeOut" "None" :!class /Script/Engine.KismetMaterialLibrary))
      (bind _output_get (Variables|Default|SetMat_FadeOut _returnvalue))
      (for _array_element (Variables|Default|GetToHide)
        (bind _asstatic_mesh_actor (Utilities|Casting|CastToStaticMeshActor _array_element))
        (Rendering|Material|SetMaterial (Variables|/Script/Engine.StaticMeshActor|GetStaticMeshComponent _asstatic_mesh_actor) 0 _output_get)))
    (:then_1
      (bind _returnvalue_2 (Rendering|Material|CreateDynamicMaterialInstance "/Game/Materials/M_FadeIn.M_FadeIn" "None" :!class /Script/Engine.KismetMaterialLibrary))
      (bind _output_get_2 (Variables|Default|SetMat_FadeIn _returnvalue_2))
      (for _array_element_2 (Variables|Default|GetToDisplay)
        (bind _asstatic_mesh_actor_2 (Utilities|Casting|CastToStaticMeshActor _array_element_2))
        (Rendering|Material|SetMaterial (Variables|/Script/Engine.StaticMeshActor|GetStaticMeshComponent _asstatic_mesh_actor_2) 0 _output_get_2)))))